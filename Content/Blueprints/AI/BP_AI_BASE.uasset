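; Base AI character Blueprint that runs the BH_AI_BASE behavior tree when play begins.
; On the GSPHealth death event it deactivates movement, calls RunBehaviorTree with no tree specified and ragdolls the mesh, which then ignores the Pawn channel.
; The GSPXpDrop component then grants the player XP, and the actor is destroyed after a short delay.
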(event OnDeath(GSPHealth)
  (params (OutKiller :type Actor%20Object%20Reference))
  (bind _mesh (Variables|Character|GetMesh))
  (Components|Activation|Deactivate (Variables|Character|GetCharacterMovement))
  (AI|RunBehaviorTree (AI|GetAIController self))
  (Physics|SetSimulatePhysics _mesh true)
  (Collision|SetCollisionResponsetoChannel _mesh "ECC_Pawn" "ECR_Ignore")
  (Class|GSPXpDropComponent|GrantPlayerwithXP (Variables|Default|GetGSPXpDrop))
  (Utilities|FlowControl|Delay 2.0)
  (Actor|DestroyActor))

(event EventBeginPlay
  (AI|RunBehaviorTree (AI|GetAIController self) "/Game/Blueprints/AI/BH_AI_BASE.BH_AI_BASE"))

(fn ConstructionScript)