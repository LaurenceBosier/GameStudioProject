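; Interactable chest prototype that shows its GSPInventory contents in a BP_ChestInventory widget.
; Interacting toggles it: opening creates the widget, switches input to game and UI, and plays the OpenChest timeline to rotate the mesh.
; Interacting again or losing interaction focus shares one close path that removes the widget, restores game-only input, hides the cursor and reverses the timeline.
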(event OnInteract(GSPInteraction)
  (params (OutRemainingInteractions :type Integer))
  (bind _returnvalue (Game|GetPlayerController 0))
  (Utilities|IsValid (Variables|Default|GetInventory%20Inst)
    (:Is%20Valid
      (Widget|RemovefromParent (Variables|Default|GetInventory%20Inst))
      (Variables|Default|SetInventory%20Inst 0)
      (Input|SetInputModeGameOnly _returnvalue)
      (Variables|/Script/Engine.PlayerController|SetbShowMouseCursor _returnvalue false)
      (bind _rotation (Timeline|OpenChest ReverseFromEnd)
        (:Update
          (Transformation|SetRelativeRotation (Variables|Default|GetStaticMesh1) (Math|Rotator|MakeRotator (* _rotation -1.0) 0.0 0.0) false false))))
    (:Is%20Not%20Valid
      (bind _returnvalue_2 (UserInterface|CreateWidget "/Game/UI/Protoypes/Inventory/BP_ChestInventory.BP_ChestInventory_C" 0 (Variables|Default|GetGSPInventory)))
      (Default|ShowInventoryContent _returnvalue_2)
      (UserInterface|Viewport|AddtoViewport _returnvalue_2 0)
      (bind _output_get (Variables|Default|SetInventory%20Inst _returnvalue_2))
      (Input|SetInputModeGameandUI (Game|GetPlayerController 0) _output_get "LockAlways" true)
      (Timeline|OpenChest PlayFromStart))))

(event OnInteractionFocusLost(GSPInteraction)
  (bind _returnvalue (Game|GetPlayerController 0))
  (Utilities|IsValid (Variables|Default|GetInventory%20Inst)
    (:Is%20Valid
      (Widget|RemovefromParent (Variables|Default|GetInventory%20Inst))
      (Variables|Default|SetInventory%20Inst 0)
      (Input|SetInputModeGameOnly _returnvalue)
      (Variables|/Script/Engine.PlayerController|SetbShowMouseCursor _returnvalue false)
      (bind _rotation (Timeline|OpenChest ReverseFromEnd)
        (:Update
          (Transformation|SetRelativeRotation (Variables|Default|GetStaticMesh1) (Math|Rotator|MakeRotator (* _rotation -1.0) 0.0 0.0) false false))))))

(fn ConstructionScript)