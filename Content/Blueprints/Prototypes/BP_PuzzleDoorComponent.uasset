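; Puzzle door component that opens its owning actor by sinking it into the ground once enough stones are gained.
; Ticking starts disabled, and each GainStone call decrements the remaining stone count.
; When the count reaches zero, it enables tick to lower the owner along local Z, then destroys the owner after a short delay.
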(event Custom|GainStone
  (bind _result (Math|Integer|DecrementInt (Variables|Default|GetNumStones))
    (:%20%20
      (if (<= _result 0)
        (Utilities|FlowControl|Sequence
          (:then_0
            (Components|Tick|SetComponentTickEnabled true))
          (:then_1
            (Utilities|FlowControl|Delay 4.0)
            (Actor|DestroyActor (Components|GetOwner))))))))

(event EventTick
  (params (DeltaSeconds :type Float%20%28single-precision%29))
  (bind _returnvalue (Components|GetOwner))
  (Utilities|IsValid _returnvalue
    (:Is%20Valid
      (Transformation|AddActorLocalOffset _returnvalue (Math|Vector|MakeVector 0.0 0.0 (* DeltaSeconds -1.5e+02)) false false))))

(event EventBeginPlay
  (Components|Tick|SetComponentTickEnabled false))