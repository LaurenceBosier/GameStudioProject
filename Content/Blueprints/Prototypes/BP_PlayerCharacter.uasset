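; Prototype player character with melee combat, weapon equipping, health and inventory.
; BeginPlay retries each tick until the HUD exists, then adds the weapon to a 3D render capture, seeds hardcoded test equipment as an editor-crash workaround, equips a sword and grants XP.
; Attacks play a montage, then call delayed damage on the child-actor weapon.
; Damage updates the HUD health bar, death ragdolls and disables input, and F runs debug stat commands.
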(event OnDeath(PlayerHealthComponent)
  (params (OutKiller :type Actor%20Object%20Reference))
  (bind _mesh (Variables|Character|GetMesh))
  ;[0.1305 1 0.3704] On Death
  (Input|DisableInput (Game|GetPlayerController 0))
  (Collision|SetCollisionProfileName _mesh "BlockAll" true :!class /Script/Engine.PrimitiveComponent)
  (Physics|SetSimulatePhysics _mesh true)
  (Development|PrintString "Debug death, restart game" true true "(R=1.000000,G=0.024522,B=0.000000,A=1.000000)" 5.0))

(event OnTakeDamage(PlayerHealthComponent)
  (params (Instigator :type Actor%20Object%20Reference) (OutDamageAmount :type Integer))
  (bind _player_hud_ref (Variables|Default|GetPlayer%20HUD%20Ref))
  (bind _playerhealthcomponent (Variables|Default|GetPlayerHealthComponent))
  ;[0.1305 1 0.3704] On Take Damage
  (Utilities|IsValid _player_hud_ref
    (:Is%20Valid
      (Default|UpdateHealthBar _player_hud_ref (Class|GSPHealthComponent|GetCurrentHealth _playerhealthcomponent) (Class|GSPHealthComponent|GetMaxHealth _playerhealthcomponent)))))

(event Custom|EquipWeapon
  (params (WeaponData :type Equipment%20Item%20Inst%20Structure%20%28by%20ref%29))
  ;[1 1 1] Equip A weapon
  (bind _asbp_weapon_master (Utilities|Casting|CastToBP_WeaponMaster (Variables|/Script/Engine.ChildActorComponent|GetChildActor (Variables|Default|GetEquipedWeapon))))
  (Default|EquipWeapon _asbp_weapon_master WeaponData)
  (AddComponent|AddAudioComponent false))

(event EventBeginPlay
  (bind _equipmentiteminst (Utilities|Struct|MakeEquipmentItemInst "/Game/Blueprints/InventoryItems/Weapons/Swords/Sword_Requiem.Sword_Requiem" 4 0 false))
  (bind _playerinventorycomponent (Variables|Default|GetPlayerInventoryComponent))
  (AddComponent|AddAudioComponent false)
  ;[1 0.09589 0] Ignore this gross loop
  (Utilities|FlowControl|DelayUntilNextTick :!label _label)
  (bind _returnvalue (Class|GSPFunctionLibrary|GetGSPGameInstance)
    (:Success
      (bind _asbp_player_hud (Utilities|Casting|CastToBP_PlayerHUD (Class|GSPMasterGameInstance|GetGamePlayHUDWidget _returnvalue))
        (:then
          (Variables|Default|SetPlayer%20HUD%20Ref _asbp_player_hud)
          ;[1 1 1] Add Weapon To Scene Capture
          (Utilities|Array|Add (Variables|/Script/Engine.SceneCaptureComponent|GetShowOnlyActors (Variables|Default|GetPlayer3DRenderCamera)) (Variables|/Script/Engine.ChildActorComponent|GetChildActor (Variables|Default|GetEquipedWeapon)))
          ;[1 1 1] Editor bug causes crash usign inherited default Items (UE 5.0.3 shit)
          (Class|GSPInventoryComponent|AddEquipmentItem _playerinventorycomponent _equipmentiteminst)
          (Class|GSPInventoryComponent|AddEquipmentItem _playerinventorycomponent (Utilities|Struct|MakeEquipmentItemInst "/Game/Blueprints/InventoryItems/Weapons/Axes/Frostbite_Axe.Frostbite_Axe" 6 0 false))
          (Class|GSPInventoryComponent|AddEquipmentItem _playerinventorycomponent (Utilities|Struct|MakeEquipmentItemInst "/Game/Blueprints/InventoryItems/Weapons/Spears/Spear_Omega.Spear_Omega" 4 0 false))
          (Class|GSPInventoryComponent|AddEquipmentItem _playerinventorycomponent (Utilities|Struct|MakeEquipmentItemInst "/Game/Blueprints/InventoryItems/Weapons/Spears/Spear_BlindJustice.Spear_BlindJustice" 8 0 false))
          (Class|GSPInventoryComponent|AddEquipmentItem _playerinventorycomponent (Utilities|Struct|MakeEquipmentItemInst "/Game/Blueprints/InventoryItems/Weapons/Swords/Sword_Gladius.Sword_Gladius" 12 0 false))
          (bind _asbp_weapon_master (Utilities|Casting|CastToBP_WeaponMaster (Variables|/Script/Engine.ChildActorComponent|GetChildActor (Variables|Default|GetEquipedWeapon))))
          (Default|EquipWeapon _asbp_weapon_master _equipmentiteminst)
          (Class|GSPXpDropComponent|GrantPlayerwithXP (Variables|Default|GetGSPXpDrop)))
        (:CastFailed
          (goto _label))))
    (:Failed
      (goto _label))))

(event EventOnJumped
  (AddComponent|AddAudioComponent false))

(event Input|ActionEvents|InputActionAttack
  (params (Key :type Key%20Structure :default "None"))
  (:Pressed
    (if (not (Variables|Default|GetInAttack))
      (Variables|Default|SetInAttack true)
      (Animation|Montage|PlayMontage (Variables|Character|GetMesh) "/Game/Assets/Characters/PlayerCharacter/Animations/SwordAndShield/SlashMontage.SlashMontage" 1.25
        (:then
          (AddComponent|AddAudioComponent false)
          (Utilities|FlowControl|Delay 0.6)
          (bind _asbp_weapon_master (Utilities|Casting|CastToBP_WeaponMaster (Variables|/Script/Engine.ChildActorComponent|GetChildActor (Variables|Default|GetEquipedWeapon))))
          (Default|DealDamage _asbp_weapon_master (Variables|Default|GetFollowCamera)))
        (:OnCompleted
          (Variables|Default|SetInAttack false))))))

(event Input|KeyboardEvents|F
  (params (Key :type Key%20Structure :default "None"))
  (bind _returnvalue (Game|GetPlayerController 0))
  ;[1 1 1] Debug Toggle Remvoe
  (:Pressed
    (Development|ExecuteConsoleCommand "Stat UNIT" _returnvalue)
    (Development|ExecuteConsoleCommand "Stat UnitGraph" _returnvalue)
    (Development|ExecuteConsoleCommand "Stat fps" _returnvalue)))

(fn ConstructionScript)