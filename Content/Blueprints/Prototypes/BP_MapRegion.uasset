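; Prototype map region actor that outlines a named area with a spline and prints a welcome message when its border is overlapped.
; The construction script rebuilds hidden box colliders along each segment, closing the loop back to the first point via GetNextLocation.
; It also centers a size-scaled name label on the points' average, which is destroyed at BeginPlay.
; Events add or remove spline points and toggle collider visibility.
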(event Custom|Add%20Spline%20Point
  (Spline|AddSplinePoint (Variables|Default|GetSpline) (Math|Vector|MakeVector 0.0 0.0 0.0) "Local" true))

(event Custom|Hide%20Colliders
  (for _array_element (Variables|RegionSettings|GetColliders)
    (Rendering|SetVisibility _array_element false false)))

(event Custom|Remove%20Spline%20Point
  (Spline|RemoveSplinePoint (Variables|Default|GetSpline) 0 true))

(event Custom|Show%20Colliders
  (for _array_element (Variables|RegionSettings|GetColliders)
    (Rendering|SetVisibility _array_element true false)))

(event EventBeginPlay
  (Components|DestroyComponent (Variables|Default|GetTextRender)))

(fn ConstructionScript
  (bind _returnvalue (Transformation|GetActorLocation))
  (bind _spline (Variables|Default|GetSpline))
  (bind _colliders (Variables|RegionSettings|GetColliders))
  (bind _returnvalue_2 (Spline|GetNumberOfSplinePoints _spline))
  (Rendering|Components|TextRender|SetWorldSize (Variables|Default|GetTextRender) (/ (Spline|GetSplineLength (Variables|Default|GetSpline)) (+ (Utilities|String|Len (Utilities|String|ToString(Text) (Variables|RegionSettings|GetRegion%20Name))) 5)))
  (Rendering|Components|TextRender|SetText (Variables|Default|GetTextRender) (Variables|RegionSettings|GetRegion%20Name))
  (LocalVariables|SetPosXSum 0.0)
  (LocalVariables|SetPosYSum 0.0)
  (for _array_element _colliders
    (Utilities|IsValid _array_element
      (:Is%20Valid
        (Components|DestroyComponent _array_element))))
  (Utilities|Array|Clear _colliders)
  (Transformation|SetActorLocation (Math|Vector|MakeVector (.x _returnvalue) (.y _returnvalue) (Variables|RegionSettings|GetZ%20Height)) false true)
  (for _index (range 0 (- _returnvalue_2 1))
    (LocalVariables|SetPosXSum (+ (LocalVariables|GetPosXSum) (.x (Spline|GetLocationatSplinePoint _spline _index "World"))))
    (LocalVariables|SetPosYSum (+ (LocalVariables|GetPosYSum) (.y (Spline|GetLocationatSplinePoint _spline _index "World"))))
    (bind _returnvalue_3 (AddComponent|AddBoxComponent true (Math|Transform|MakeTransform (.Location (CallFunction|GetNextLocation _index (Variables|Default|GetSpline))) (.Rotation (CallFunction|GetNextLocation _index (Variables|Default|GetSpline))) "1.000000,1.000000,1.000000")))
    (Utilities|Array|Add (Variables|RegionSettings|GetColliders) _returnvalue_3)
    (Rendering|SetVisibility _returnvalue_3 false false)
    (Class|BoxComponent|SetLineThickness _returnvalue_3 15.0)
    (Components|Box|SetBoxExtent _returnvalue_3 (Math|Vector|MakeVector (Math|Conversions|ToFloat(Integer) (.Distane (CallFunction|GetNextLocation _index (Variables|Default|GetSpline)))) 25.0 (/ (Variables|RegionSettings|GetZ%20Height) 2.0)) false)
    (Collision|BindEventtoOnComponentBeginOverlap _returnvalue_3 (EventDispatchers|CreateEvent :!event BPMapRegionAutoGenFunc)))
  (Transformation|SetWorldLocation (Variables|Default|GetTextRender) (Math|Vector|MakeVector (/ (LocalVariables|GetPosXSum) _returnvalue_2) (/ (LocalVariables|GetPosYSum) _returnvalue_2) (Variables|RegionSettings|GetZ%20Height)) false false))

(fn BPMapRegionAutoGenFunc
  (params (OverlappedComponent :type Primitive%20Component%20Object%20Reference) (OtherActor :type Actor%20Object%20Reference) (OtherComp :type Primitive%20Component%20Object%20Reference) (OtherBodyIndex :type Integer) (bFromSweep :type Boolean) (SweepResult :type Hit%20Result%20Structure%20%28by%20ref%29))
  (Development|PrintString (Utilities|String|Append "Welcome to: " (Utilities|String|ToString(Text) (Variables|RegionSettings|GetRegion%20Name))) true true "(R=0.190525,G=1.000000,B=0.000000,A=1.000000)" 1e+01)
  (return))

(fn GetNextLocation
  (params (index :type Integer) (InSpline :type Spline%20Component%20Object%20Reference))
  (bind _returnvalue (Spline|GetLocationatSplinePoint InSpline index "World"))
  (bind _returnvalue_2 (+ index 1))
  (bind _z_height (Variables|RegionSettings|GetZ%20Height))
  (bind _returnvalue_3 (Spline|GetLocationatSplinePoint InSpline 0 "World"))
  (bind _returnvalue_4 (Spline|GetLocationatSplinePoint InSpline _returnvalue_2 "World"))
  (bind _returnvalue_5 (Spline|GetLocationatSplinePoint InSpline index "World"))
  (bind _returnvalue_6 (/ _z_height 2.0))
  (bind _returnvalue_7 (- _returnvalue_6 1e+02))
  (bind _returnvalue_8 (- _returnvalue_3 _returnvalue_5))
  (bind _returnvalue_9 (- _returnvalue_4 _returnvalue))
  (bind _returnvalue_10 (/ _returnvalue_8 2))
  (bind _returnvalue_11 (/ _returnvalue_9 2))
  (bind _returnvalue_12 (+ _returnvalue_5 _returnvalue_10))
  (bind _returnvalue_13 (+ _returnvalue _returnvalue_11))
  (if (> (+ index 1) (- (Spline|GetNumberOfSplinePoints InSpline) 1))
    (return (Math|Vector|MakeVector (.x _returnvalue_12) (.y _returnvalue_12) _returnvalue_7) (Math|Rotator|FindLookatRotation _returnvalue_5 _returnvalue_3) (/ (Math|Float|Truncate (Math|Vector|VectorLength (- _returnvalue_3 _returnvalue_5))) 2))
    (else
      (return (Math|Vector|MakeVector (.x _returnvalue_13) (.y _returnvalue_13) _returnvalue_7) (Math|Rotator|FindLookatRotation _returnvalue _returnvalue_4) (/ (Math|Float|Truncate (Math|Vector|VectorLength (- _returnvalue_4 _returnvalue))) 2)))))