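; Prototype weapon pickup actor that adds a weapon to the player's inventory when interacted with.
; The construction script sets its mesh and scale from the equipment data asset in WeaponDetails, and BeginPlay enables physics simulation on that mesh.
; On GSPInteraction interact, it finds player character 0's GSPInventoryComponent, adds WeaponDetails as an equipment item and destroys itself.
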(event OnInteract(GSPInteraction)
  (params (OutRemainingInteractions :type Integer))
  (bind _returnvalue (Class|GSPFunctionLibrary|GetGSPComponentfromActor (Game|GetPlayerCharacter 0) "/Script/GameStudioProject.GSPInventoryComponent")
    (:Success
      (Class|GSPInventoryComponent|AddEquipmentItem _returnvalue (Variables|Default|GetWeaponDetails))
      (Actor|DestroyActor))))

(event EventBeginPlay
  (Physics|SetSimulatePhysics (Variables|Default|GetStaticMesh) true))

(fn ConstructionScript
  (bind _weapondetails (Variables|Default|GetWeaponDetails))
  (Components|StaticMesh|SetStaticMesh (Variables|Default|GetStaticMesh) (Variables|/Script/GameStudioProject.GSPInventoryItem|GetItemMesh (.equipmentdataasset _weapondetails)))
  (Transformation|SetActorScale3D (Math|Conversions|ToVector(Float) (Variables|/Script/GameStudioProject.GSPInventoryItem|GetPickupScale (.equipmentdataasset _weapondetails)))))