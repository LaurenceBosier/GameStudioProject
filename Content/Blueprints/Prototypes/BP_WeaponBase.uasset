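; BP_WeaponBase is a prototype base Blueprint for weapons, showing a mesh taken from equipment data.
; Its construction script reads the ItemMesh from the EquipmentDataAsset inside WeaponDetails and, if valid, applies it to the StaticMesh component.
; The other item fields, such as name, value, type and rarity, are unused, and the event graph holds no active logic.
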(event EventBeginPlay)

(event EventTick
  (params (DeltaSeconds :type Float%20%28single-precision%29)))

(fn ConstructionScript
  (bind _weapondetails (Variables|Default|GetWeaponDetails))
  (bind _equipmentdataasset (Utilities|Struct|BreakEquipmentItemInst _weapondetails))
  (bind _itemmesh (Variables|/Script/GameStudioProject.GSPInventoryItem|GetItemMesh _equipmentdataasset))
  (Utilities|IsValid _itemmesh
    (:Is%20Valid
      (Components|StaticMesh|SetStaticMesh (Variables|Default|GetStaticMesh) _itemmesh))))