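; BP_InteractableTest is a prototype actor for testing interaction, health and XP rewards through GSP components.
; Each interaction prints the remaining interaction count and has GSPXpDrop grant the player XP.
; The last interaction destroys the actor, and death reported by GSPHealth grants XP before destroying it.
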(event OnInteract(GSPInteraction)
  (params (OutRemainingInteractions :type Integer))
  (Development|PrintString (Utilities|String|Append "Remaining Interactions: " (Utilities|String|ToString(Integer) OutRemainingInteractions)))
  (Class|GSPXpDropComponent|GrantPlayerwithXP (Variables|Default|GetGSPXpDrop)))

(event OnDeath(GSPHealth)
  (params (OutKiller :type Actor%20Object%20Reference))
  (Class|GSPXpDropComponent|GrantPlayerwithXP (Variables|Default|GetGSPXpDrop))
  (Actor|DestroyActor))

(event OnLastInteraction(GSPInteraction)
  (Actor|DestroyActor))

(fn ConstructionScript)