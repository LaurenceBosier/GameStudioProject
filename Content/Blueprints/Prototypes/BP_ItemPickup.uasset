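; BP_ItemPickup is a prototype world pickup for equipment, configured through the data asset in its WeaponDetails.
; The construction script applies the asset's mesh and pickup scale to StaticMesh and enables physics simulation when that mesh is valid.
; On GSPInteraction OnInteract, Equipment-category items are added to player 0's inventory component, and the actor destroys itself only if the add succeeds.
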(event OnInteract(GSPInteraction)
  (params (OutRemainingInteractions :type Integer))
  (bind _asgame_studio_project_character (Utilities|Casting|CastToGameStudioProjectCharacter (Game|GetPlayerCharacter 0)))
  (switch Utilities|FlowControl|Switch|SwitchonEItemCategory (Variables|/Script/GameStudioProject.GSPInventoryItem|GetItemCategory (.equipmentdataasset (Variables|Default|GetWeaponDetails)))
    (:Equipment
      (bind _returnvalue (Class|GSPInventoryComponent|AddEquipmentItem (Variables|/Script/GameStudioProject.GameStudioProjectCharacter|GetPlayerInventoryComponent _asgame_studio_project_character) (Variables|Default|GetWeaponDetails)))
      (if _returnvalue
        (Actor|DestroyActor)))))

(fn ConstructionScript
  (bind _weapondetails (Variables|Default|GetWeaponDetails))
  (bind _equipmentdataasset (Utilities|Struct|BreakEquipmentItemInst _weapondetails))
  (bind _itemmesh (Variables|/Script/GameStudioProject.GSPInventoryItem|GetItemMesh _equipmentdataasset))
  (Utilities|IsValid _itemmesh
    (:Is%20Valid
      (Components|StaticMesh|SetStaticMesh (Variables|Default|GetStaticMesh) _itemmesh)
      (Transformation|SetWorldScale3D (Variables|Default|GetStaticMesh) (Math|Conversions|ToVector(Float) (Variables|/Script/GameStudioProject.GSPInventoryItem|GetPickupScale _equipmentdataasset)))
      (Physics|SetSimulatePhysics (Variables|Default|GetStaticMesh) true))))