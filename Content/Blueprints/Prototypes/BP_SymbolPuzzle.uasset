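; BP_SymbolPuzzle is a prototype interactable symbol stone that counts toward opening a linked puzzle door.
; On its last GSP interaction, it finds the BP_PuzzleDoorComponent on OwningDoor and calls GainStone.
; It then applies its Symbol material to slot 1 of the static mesh on the referenced Mesh and destroys itself.
; The construction script is empty, with mesh and material setup left unconnected.
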(event OnLastInteraction(GSPInteraction)
  (bind _owningdoor (Variables|Default|GetOwningDoor))
  (Utilities|IsValid _owningdoor
    (:Is%20Valid
      (bind _returnvalue (Class|GSPFunctionLibrary|GetGSPComponentfromActor _owningdoor "/Game/Blueprints/Prototypes/BP_PuzzleDoorComponent.BP_PuzzleDoorComponent_C")
        (:Success
          (Default|GainStone _returnvalue)
          (Rendering|Material|SetMaterial (Actor|GetComponentbyClass (Variables|Default|GetMesh) "/Script/Engine.StaticMeshComponent") 1 "/Game/SymbolPuzzle/Meshes/Symbol.Symbol")
          (Actor|DestroyActor))))))

(fn ConstructionScript)