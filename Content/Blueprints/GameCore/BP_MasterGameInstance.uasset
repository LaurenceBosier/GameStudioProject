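; BP_MasterGameInstance is the game instance Blueprint that relays interaction popup and player progression events to the UI.
; Interaction events set or remove text on the BP_PlayerHUD gameplay widget.
; XP gain and level-up events share a path refreshing level and XP in BP_PlayerMenu, and each updates the HUD XP bar, printing a failure message if the HUD cast fails.
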(event EventOnAddInteractionPopup
  (params (OutPopupMessage :type EInteractionPopupMessage%20Enum :default "Interact"))
  (bind _asbp_player_hud (Utilities|Casting|CastToBP_PlayerHUD (Class|GSPMasterGameInstance|GetGamePlayHUDWidget)))
  (Default|SetInteractionText _asbp_player_hud OutPopupMessage))

(event EventOnRemoveInteractionPopup
  (bind _asbp_player_hud (Utilities|Casting|CastToBP_PlayerHUD (Class|GSPMasterGameInstance|GetGamePlayHUDWidget)))
  (Default|RemoveInteractionText _asbp_player_hud))

(event EventOnGainXp
  (params (OutXpAmount :type Integer))
  (Utilities|FlowControl|Sequence
    (:then_0
      (bind _asbp_player_menu (Utilities|Casting|CastToBP_PlayerMenu (Class|GSPMasterGameInstance|GetMenuWidget)))
      (Default|SetPlayerLevelandXp _asbp_player_menu (Class|GSPMasterGameInstance|GetCurrentPlayerLevel) (Class|GSPMasterGameInstance|GetCurrentPlayerLevelXp) (Class|GSPMasterGameInstance|GetRequiredXpforLevelUp)))
    (:then_1
      (bind _asbp_player_hud (Utilities|Casting|CastToBP_PlayerHUD (Class|GSPMasterGameInstance|GetGamePlayHUDWidget))
        (:then
          (Default|UpdateXPBar _asbp_player_hud (Class|GSPMasterGameInstance|GetCurrentPlayerLevelXp) (Class|GSPMasterGameInstance|GetRequiredXpforLevelUp)))
        (:CastFailed
          (Development|PrintString "Failed"))))))

(event EventOnLevelUp
  (params (OutNewLevel :type Integer))
  (Utilities|FlowControl|Sequence
    (:then_0
      (bind _asbp_player_menu (Utilities|Casting|CastToBP_PlayerMenu (Class|GSPMasterGameInstance|GetMenuWidget)))
      (Default|SetPlayerLevelandXp _asbp_player_menu (Class|GSPMasterGameInstance|GetCurrentPlayerLevel) (Class|GSPMasterGameInstance|GetCurrentPlayerLevelXp) (Class|GSPMasterGameInstance|GetRequiredXpforLevelUp)))
    (:then_1
      (bind _asbp_player_hud (Utilities|Casting|CastToBP_PlayerHUD (Class|GSPMasterGameInstance|GetGamePlayHUDWidget))
        (:then
          (Default|UpdateXPBar _asbp_player_hud (Class|GSPMasterGameInstance|GetCurrentPlayerLevelXp) (Class|GSPMasterGameInstance|GetRequiredXpforLevelUp)))
        (:CastFailed
          (Development|PrintString "Failed"))))))