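; Master weapon actor that displays an equipped item from its equipment data asset, hardcoded to Hellhunter_Axe on BeginPlay.
; EquipWeapon marks the item struct as equipped and, if its data asset is valid, swaps the weapon mesh.
; It then resets the actor's relative transform and teleports it to the asset's spawn offset.
; The construction script disables collision on all child static mesh components.
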(event Custom|Equip%20Weapon
  (params (WeaponData :type Equipment%20Item%20Inst%20Structure%20%28by%20ref%29))
  (bind _structout (Utilities|Struct|SetmembersinEquipmentItemInst WeaponData true))
  (Variables|Default|SetWeaponData _structout)
  (Utilities|IsValid (.equipmentdataasset (Variables|Default|GetWeaponData))
    (:Is%20Valid
      (if (.isequipped (Variables|Default|GetWeaponData))
        (Components|StaticMesh|SetStaticMesh (Variables|Default|GetWeaponMesh) (Variables|/Script/GameStudioProject.GSPInventoryItem|GetItemMesh (.equipmentdataasset (Variables|Default|GetWeaponData))))
        (Transformation|SetActorRelativeTransform (Math|Transform|MakeTransform "0, 0, 0" "0, 0, 0" "1.000000,1.000000,1.000000") false true)
        (Transformation|SetActorRelativeTransform (Variables|/Script/GameStudioProject.GSPInventoryItem|GetSpawnOffset (.equipmentdataasset (Variables|Default|GetWeaponData))) false true)))))

(event EventBeginPlay
  (CallFunction|EquipWeapon (Utilities|Struct|MakeEquipmentItemInst "/Game/Blueprints/InventoryItems/Weapons/Axes/Hellhunter_Axe.Hellhunter_Axe" 0 0 false)))

(fn ConstructionScript
  (for _array_element (Components|GetChildrenComponents (Variables|Default|GetDefaultSceneRoot) true)
    (bind _asstatic_mesh_component (Utilities|Casting|CastToStaticMeshComponent _array_element))
    (Collision|SetCollisionEnabled _asstatic_mesh_component "NoCollision")))