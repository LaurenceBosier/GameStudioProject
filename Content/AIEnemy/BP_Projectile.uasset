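; BP_Projectile is a projectile that damages an actor when its box overlaps it, then destroys itself.
; With a valid TargetDMG, typically for AI shooters, it hits only that target; otherwise it hits actors whose AIEnemy component AllyOrEnemy differs from the DamageCauser's.
; Each branch uses DoOnce to apply damage and report a damage event, though the untargeted branch reports the invalid TargetDMG.
; Destruction spawns an explosion emitter at its location.
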(event OnComponentBeginOverlap(Box)
  (params (OverlappedComponent :type Primitive%20Component%20Object%20Reference) (OtherActor :type Actor%20Object%20Reference) (OtherComp :type Primitive%20Component%20Object%20Reference) (OtherBodyIndex :type Integer) (bFromSweep :type Boolean) (SweepResult :type Hit%20Result%20Structure%20%28by%20ref%29))
  (bind _targetdmg (Variables|Default|GetTargetDMG))
  (Variables|Default|GetTargetDMG
    (:then
      ;[1 1 1] Logic is the owner projectile has the AIControler, example The enemy
      (if (== OtherActor _targetdmg)
        (Utilities|IsValid _targetdmg
          (:Is%20Valid
            (Utilities|FlowControl|DoOnce false
              (:Completed
                (bind _returnvalue (Game|Damage|ApplyDamage (Variables|Default|GetTargetDMG) (Variables|Default|GetBase%20Damage) 0 (Variables|Default|GetDamage%20Causer)))
                (Class|AISenseDamage|ReportDamageEvent (Variables|Default|GetTargetDMG) (Variables|Default|GetDamage%20Causer) _returnvalue (Transformation|GetActorLocation) "0, 0, 0" "None")
                (Actor|DestroyActor)))))))
    (:else
      ;[1 1 1] Logic If the owner does not have AI Controler, example the player character
      (if (!= (Variables|/Game/AIEnemy/C_AIEnemyComponet.C_AIEnemyComponet_C|GetAllyOrEnemy (CallFunction|GetAIEnemyComp OtherActor)) (Variables|/Game/AIEnemy/C_AIEnemyComponet.C_AIEnemyComponet_C|GetAllyOrEnemy (CallFunction|GetAIEnemyComp (Variables|Default|GetDamage%20Causer))))
        (Utilities|FlowControl|DoOnce false
          (:Completed
            (Game|Damage|ApplyDamage OtherActor (Variables|Default|GetBase%20Damage) 0 (Variables|Default|GetDamage%20Causer))
            (Class|AISenseDamage|ReportDamageEvent (Variables|Default|GetTargetDMG) (Variables|Default|GetDamage%20Causer) 0.0 (Transformation|GetActorLocation) "0, 0, 0" "None")
            (Actor|DestroyActor)))))))

(event EventDestroyed
  (Effects|SpawnEmitteratLocation "/Game/AIEnemy/Demo/StarterContent/Particles/P_Explosion.P_Explosion" (Transformation|GetActorLocation)))

(fn ConstructionScript)